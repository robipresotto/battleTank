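; Player-controllable tank pawn Blueprint that wires input to aiming and movement components and sets up a health bar widget.
; On BeginPlay it hands the barrel and turret to TankAiming, both tracks to TankMovement, and itself to the health bar widget.
; Aim axes rotate the azimuth gimbal and spring arm, scaled by delta time, while fire and move inputs forward to those two components.
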(event `self.ReceiveBeginPlay`
  (`tankAimingComponent.Initialise` (`self.tankAiming`) (`self.Barrel`) (`self.Turret`))
  (`TankMovementComponent.initialise` (`self.TankMovement`) (`self.LeftTrack`) (`self.RightTrack`))
  (`self.InitialiseHealthBarWidget`))

(event `InputAxis|AimAzimuth`
  (params (AxisValue :type "Float (single-precision)"))
  ;[1 1 1] Aim input binding
  (`SceneComponent.K2_AddLocalRotation` (`self.Azimuth Gimbal`) (`KismetMathLibrary.MakeRotator` 0.0 0.0 (* AxisValue (`GameplayStatics.GetWorldDeltaSeconds`) 100.0)) false false))

(event `InputAxis|AimElevation`
  (params (AxisValue :type "Float (single-precision)"))
  ;[1 1 1] Aim input binding
  (`SceneComponent.K2_AddLocalRotation` (`self.SpringArm`) (`KismetMathLibrary.MakeRotator` 0.0 (* 100.0 AxisValue (`GameplayStatics.GetWorldDeltaSeconds`))) false false))

(event `InputAction|Fire`
  (params (Key :type "Key Structure" :default "AnyKey"))
  ;[1 1 1] Fire Action
  (:`Pressed`
    (`tankAimingComponent.Fire` (`self.tankAiming`))))

(event `InputAxis|Move Forward`
  (params (AxisValue :type "Float (single-precision)"))
  ;[1 1 1] Movement input binding
  (`TankMovementComponent.intendMoveForward` (`self.TankMovement`) AxisValue))

(event `InputAxis|Move Right`
  (params (AxisValue :type "Float (single-precision)"))
  ;[1 1 1] Movement input binding
  (`TankMovementComponent.intendTurnRight` (`self.TankMovement`) AxisValue))

(fn `InitialiseHealthBarWidget`
  (bind _ashealth_bar (cast `/Game/Blueprints/healthBar` (`WidgetComponent.GetUserWidgetObject` (`self.Widget`)))
    (:`then`
      (set `/Game/Blueprints/healthBar.tank` self _ashealth_bar))
    (:`CastFailed`
      _))
  (return))

(fn `UserConstructionScript`)